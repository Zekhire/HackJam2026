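; Combat component for a Character that handles health, melee attacks, dash, jump and weapon swapping, adding a health bar for player-controlled owners.
; A weapon factory supplies the default weapon, and each weapon's data sets its socket, attack montage and locomotion AnimBP.
; Dropped non-default weapons gain an acquirable component, while collision toggles control overlap events and deactivation clears the hit list.
; Montage-length delays gate attack and dash, and lethal damage ragdolls the owner.
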(event `Attack`
  (bind (_weapondata_mindamage _weapondata_maxdamage _weapondata_model _weapondata_components _weapondata_attackanimation) (break `/Game/Blueprints/Weapons/UtilWeaponData` (`/Game/Blueprints/Weapons/BP_Weapon.weaponData` (`self.weapon`))))
  (if (`self.isAlive`)
    (if (`NavMovementComponent.IsFalling` (`Pawn.GetMovementComponent` (`self.ownerCharacter`)))
      _
      (elif (`self.canAttack`)
        (if (`KismetSystemLibrary.IsValid` (`self.weapon`))
          (set `self.canAttack` false)
          (`CharacterMovementComponent.DisableMovement` (`Character.CharacterMovement` (`self.ownerCharacter`)))
          (`KismetSystemLibrary.PrintText` (`KismetTextLibrary.Conv_ObjectToText` _weapondata_attackanimation))
          (bind _returnvalue (`Character.PlayAnimMontage` (`self.ownerCharacter`) _weapondata_attackanimation 1.5 "None"))
          (`KismetSystemLibrary.Delay` (/ _returnvalue 1.5))
          (`CharacterMovementComponent.SetMovementMode` (`Character.CharacterMovement` (`self.ownerCharacter`)) "MOVE_Walking" 0)
          (`KismetSystemLibrary.Delay` 0.2)
          (set `self.canAttack` true))))))

(event `self.ReceiveBeginPlay`
  (set `self.health` (`self.maxHealth`))
  (bind _ascharacter (cast `Character` (`KismetSystemLibrary.GetOuterObject` self)))
  (bind _output_get (set `self.ownerCharacter` _ascharacter))
  (if (`Pawn.IsPlayerControlled` _output_get)
    (bind _returnvalue (`|CreateWidget` "/Game/Widgets/WBP_HealthBar.WBP_HealthBar_C" (`GameplayStatics.GetPlayerController` 0)))
    (`UserWidget.AddToViewport` _returnvalue 0))
  (`self.CreateDefaultWeapon`)
  (add `Actor.OnTakeAnyDamage` _output_get (delegate `Event Any Damage`)))

(event `Event Any Damage`
  (params (DamagedActor :type "Actor Object Reference") (Damage :type "Float (single-precision)") (DamageType :type "DamageType Object Reference") (InstigatedBy :type "Controller Object Reference") (DamageCauser :type "Actor Object Reference"))
  (bind _ownercharacter (`self.ownerCharacter`))
  (bind _capsulecomponent (`Character.CapsuleComponent` _ownercharacter))
  (bind _mesh (`Character.Mesh` _ownercharacter))
  (if (`self.isAlive`)
    (bind _output_get (set `self.health` (- (`self.health`) Damage)))
    (if (<= _output_get 0.0)
      (set `self.health` 0.0)
      (set `self.isAlive` false)
      (`PrimitiveComponent.SetSimulatePhysics` _mesh true)
      (`PrimitiveComponent.SetCollisionResponseToChannel` _mesh "ECC_Pawn" "ECR_Ignore")
      (`PrimitiveComponent.SetCollisionEnabled` _capsulecomponent "NoCollision")
      (`PrimitiveComponent.SetCollisionResponseToChannel` _capsulecomponent "ECC_Pawn" "ECR_Ignore")
      (`KismetSystemLibrary.PrintString` "dead"))))

(event `TakeItem`
  (params (Item :type "/Game/Blueprints/Weapons/BP_Item Object Reference"))
  (bind _asbp_weapon (cast `/Game/Blueprints/Weapons/BP_Weapon` Item))
  (`self.ChangeWeapon` _asbp_weapon))

(event `DropWeapon`
  (bind _weapon (`self.weapon`))
  (`/Engine/EditorBlueprintResources/StandardMacros.IsValid` _weapon
    (:`Is Valid`
      (`Actor.K2_DetachFromActor` _weapon "KeepWorld" "KeepRelative" "KeepRelative")
      (bind _returnvalue (`|AddComponentByClass` (`self.weapon`) "/Game/Blueprints/Weapons/Components/BPC_Acquirable.BPC_Acquirable_C"))
      (`/Game/Blueprints/Weapons/Components/BPC_Acquirable.AcquirableAnimation` _returnvalue))))

(event `ChangeWeapon`
  (params (newWeapon :type "/Game/Blueprints/Weapons/BP_Weapon Object Reference"))
  (if (!= (`self.defaultWeapon`) (`self.weapon`))
    (`self.DropWeapon`))
  (`self.WeaponCollisionDeactivation`)
  (`self.SetWeapon` newWeapon))

(event `Unarm`
  (if (!= (`self.defaultWeapon`) (`self.weapon`))
    (`self.ChangeWeapon` (`self.defaultWeapon`))))

(event `SetWeapon`
  (params (newWeapon :type "/Game/Blueprints/Weapons/BP_Weapon Object Reference"))
  (bind (_weapondata_mindamage _weapondata_maxdamage _weapondata_model _weapondata_components _weapondata_attackanimation _weapondata_animlocomotion _weapondata_socket) (break `/Game/Blueprints/Weapons/UtilWeaponData` (`/Game/Blueprints/Weapons/BP_Weapon.weaponData` (`self.weapon`))))
  (bind (_weapondata_mindamage_2 _weapondata_maxdamage_2 _weapondata_model_2 _weapondata_components_2 _weapondata_attackanimation_2 _weapondata_animlocomotion_2) (break `/Game/Blueprints/Weapons/UtilWeaponData` (`/Game/Blueprints/Weapons/BP_Weapon.weaponData` (`self.weapon`))))
  (`/Engine/EditorBlueprintResources/StandardMacros.IsValid` newWeapon
    (:`Is Valid`
      (`Actor.SetOwner` newWeapon (`self.ownerCharacter`))
      (bind _output_get (set `self.weapon` newWeapon))
      (`Actor.K2_AttachToComponent` _output_get (`Character.Mesh` (`self.ownerCharacter`)) _weapondata_socket "SnapToTarget" "SnapToTarget" "SnapToTarget" true)
      (`SkeletalMeshComponent.SetAnimInstanceClass` (`Character.Mesh` (`self.ownerCharacter`)) _weapondata_animlocomotion_2))))

(event `Dash`
  (bind _ownercharacter (`self.ownerCharacter`))
  (bind _charactermovement (`Character.CharacterMovement` _ownercharacter))
  (if (`self.canDash`)
    (if (not (`NavMovementComponent.IsFalling` (`Character.CharacterMovement` (`self.ownerCharacter`))))
      (set `self.canDash` false)
      (set `self.canAttack` false)
      (set `self.canJump` false)
      (`Controller.SetIgnoreMoveInput` (`PlayerState.GetPlayerController` (`Pawn.PlayerState` _ownercharacter)) true)
      (`CharacterMovementComponent.DisableMovement` _charactermovement)
      (`CharacterMovementComponent.SetMovementMode` _charactermovement "MOVE_Walking" 0)
      (`Character.LaunchCharacter` (`self.ownerCharacter`) (* (`SceneComponent.GetForwardVector` (`Actor.RootComponent` _ownercharacter)) 1500.0) false false)
      (bind _returnvalue (`Character.PlayAnimMontage` (`self.ownerCharacter`) "/Game/Animations/AnimMontages/SprintingForwardRoll_UE_Montage.SprintingForwardRoll_UE_Montage" 1.0 "None"))
      (`NiagaraFunctionLibrary.SpawnSystemAtLocation` null (`Actor.K2_GetActorLocation` (`self.ownerCharacter`)) (`KismetMathLibrary.Conv_VectorToRotator` (* (`KismetMathLibrary.GetForwardVector` (`Actor.K2_GetActorRotation` (`self.ownerCharacter`))) -1.0)))
      (`KismetSystemLibrary.Delay` (* _returnvalue 0.8))
      (`Controller.SetIgnoreMoveInput` (`PlayerState.GetPlayerController` (`Pawn.PlayerState` (`self.ownerCharacter`))) false)
      (set `self.canAttack` true)
      (set `self.canJump` true)
      (set `self.canDash` true))))

(event `Key|LeftMouseButton`
  (params (Key :type "Key Structure"))
  (:`Pressed`
    (`self.Attack`)))

(event `Key|Z`
  (params (Key :type "Key Structure"))
  (:`Pressed`
    (`self.Dash`)))

(event `ClearHittedActors`
  (`KismetArrayLibrary.Array_Clear` (`self.HittedActors`)))

(event `EnhancedInput|/Game/Input/Actions/IA_Jump`
  (params (ActionValue :type Boolean) (ElapsedSeconds :type "Float (double-precision)") (TriggeredSeconds :type "Float (double-precision)") (InputAction :type "InputAction Object Reference" :default "/Game/Input/Actions/IA_Jump.IA_Jump"))
  (bind _ownercharacter (`self.ownerCharacter`))
  (:`Started`
    (if (`self.canJump`)
      (`Character.Jump` _ownercharacter)))
  (:`Completed`
    (`Character.StopJumping` _ownercharacter)))

(event `CreateDefaultWeapon`
  (bind _returnvalue (`|GenericCreateObject` "/Game/Blueprints/Weapons/OBJ_WeaponFactory.OBJ_WeaponFactory_C"))
  (bind (_value _returnvalue_2) (`BlueprintMapLibrary.Map_Find` (`/Game/Blueprints/Weapons/OBJ_WeaponFactory.Weapons` _returnvalue) (`|GetEnumeratorNameAsString` (`self.defaultWeaponType`))))
  (if _returnvalue_2
    (bind _returnvalue_3 (`|SpawnActorFromClass` "/Game/Blueprints/Weapons/BP_Weapon.BP_Weapon_C" (`KismetMathLibrary.MakeTransform` (0.0 0.0 0.0)) "Undefined" "MultiplyWithRoot" (`self.ownerCharacter`) _value null))
    (bind _output_get (set `self.defaultWeapon` _returnvalue_3))
    (`self.SetWeapon` _output_get)))

(event `WeaponCollisionDeactivation`
  (bind _returnvalue (`Actor.GetComponentByClass` (`/Game/Blueprints/Weapons/BP_Weapon.weaponModel` (`self.weapon`)) "/Script/Engine.ShapeComponent"))
  (`/Engine/EditorBlueprintResources/StandardMacros.IsValid` _returnvalue
    (:`Is Valid`
      (set `PrimitiveComponent.bGenerateOverlapEvents` false _returnvalue))
    (:`Is Not Valid`
      _))
  (`self.ClearHittedActors`))

(event `WeaponCollisionActivation`
  (bind _returnvalue (`Actor.GetComponentByClass` (`/Game/Blueprints/Weapons/BP_Weapon.weaponModel` (`self.weapon`)) "/Script/Engine.ShapeComponent"))
  (`/Engine/EditorBlueprintResources/StandardMacros.IsValid` _returnvalue
    (:`Is Valid`
      (set `PrimitiveComponent.bGenerateOverlapEvents` true _returnvalue))
    (:`Is Not Valid`)))