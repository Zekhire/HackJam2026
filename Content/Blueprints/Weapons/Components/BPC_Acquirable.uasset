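; Component that makes its owning BP_Item a world pickup that players can take with E.
; On BeginPlay it adds a sphere collider to the item, which enables or disables item input as players enter or leave.
; E finds which local player pressed it, passes the item to their BPC_CombatComponent, then destroys the collider and itself.
; AcquirableAnimation uses looping timers and a curve to spin and bob the item.
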(event `OnComponentBeginOverlap_Event`
  (params (OverlappedComponent :type "PrimitiveComponent Object Reference") (OtherActor :type "Actor Object Reference") (OtherComp :type "PrimitiveComponent Object Reference") (OtherBodyIndex :type Integer) (bFromSweep :type Boolean) (SweepResult :type "HitResult Structure (by ref)"))
  (bind _asbp_player (cast `/Game/CustomCharacters/SkeletalMeshes/BP_Player` OtherActor))
  (`Actor.EnableInput` (`self.ownerItem`) (`PlayerState.GetPlayerController` (`Pawn.PlayerState` _asbp_player))))

(event `self.ReceiveBeginPlay`
  (bind _asbp_item (cast `/Game/Blueprints/Weapons/BP_Item` (`KismetSystemLibrary.GetOuterObject` self)))
  (bind _output_get (set `self.ownerItem` _asbp_item))
  (`Actor.SetOwner` _output_get null)
  (bind _returnvalue (`|AddComponentByClass` :`self` _output_get :`Class` "/Script/Engine.SphereComponent"))
  (bind _output_get_2 (set `self.collider` _returnvalue))
  (`SphereComponent.SetSphereRadius` _output_get_2 100.0 false)
  (add `PrimitiveComponent.OnComponentBeginOverlap` _output_get_2 (delegate `OnComponentBeginOverlap_Event`))
  (add `PrimitiveComponent.OnComponentEndOverlap` _output_get_2 (delegate `OnComponentEndOverlap_Event`)))

(event `OnComponentEndOverlap_Event`
  (params (OverlappedComponent :type "PrimitiveComponent Object Reference") (OtherActor :type "Actor Object Reference") (OtherComp :type "PrimitiveComponent Object Reference") (OtherBodyIndex :type Integer))
  (bind _asbp_player (cast `/Game/CustomCharacters/SkeletalMeshes/BP_Player` OtherActor))
  (`Actor.DisableInput` (`self.ownerItem`) (`PlayerState.GetPlayerController` (`Pawn.PlayerState` _asbp_player))))

(event `Key|E`
  (params (Key :type "Key Structure"))
  (:`Pressed`
    (for _index (range (`GameplayStatics.GetNumLocalPlayerControllers`))
      (if (`PlayerController.WasInputKeyJustPressed` (`GameplayStatics.GetPlayerController` _index) "E")
        (`self.TakeItem` (`GameplayStatics.GetPlayerCharacter` _index))))))

(event `TakeItem`
  (params (character :type "Character Object Reference"))
  (`/Game/Blueprints/Weapons/Components/BPC_CombatComponent.TakeItem` (`Actor.GetComponentByClass` character "/Game/Blueprints/Weapons/Components/BPC_CombatComponent.BPC_CombatComponent_C") (`self.ownerItem`))
  (`/Game/Blueprints/Weapons/BP_Item.DestroyComponent` (`self.ownerItem`) (`self.collider`))
  (`self.K2_DestroyComponent`))

(event `AcquirableAnimation`
  (bind _returnvalue (`KismetSystemLibrary.K2_SetTimerDelegate` (delegate `FinishFunc`) 5.0 true))
  (`KismetSystemLibrary.K2_SetTimerDelegate` (delegate `UpdateFunc`) (`GameplayStatics.GetWorldDeltaSeconds`) true))

(event `FinishFunc`)

(event `UpdateFunc`
  (bind (_returnvalue_roll _returnvalue_pitch) (`KismetMathLibrary.BreakRotator` (`Actor.K2_GetActorRotation` (`self.ownerItem`))))
  (bind (_returnvalue_x _returnvalue_y _returnvalue_z) (`KismetMathLibrary.BreakVector` (`Actor.K2_GetActorLocation` (`self.ownerItem`))))
  (bind _returnvalue (`KismetMathLibrary.GetRuntimeFloatCurveValue` (`self.curve`) (`KismetSystemLibrary.K2_GetTimerElapsedTimeHandle` (stale `AcquirableAnimation` _returnvalue))))
  (`Actor.K2_SetActorRelativeRotation` (`self.ownerItem`) (`KismetMathLibrary.MakeRotator` _returnvalue_roll _returnvalue_pitch (* _returnvalue 360.0)) false false)
  (`Actor.K2_SetActorLocation` (`self.ownerItem`) (`KismetMathLibrary.MakeVector` _returnvalue_x _returnvalue_y (+ _returnvalue_z (* (`KismetMathLibrary.DegSin` (* _returnvalue 360.0)) 0.2))) false false))