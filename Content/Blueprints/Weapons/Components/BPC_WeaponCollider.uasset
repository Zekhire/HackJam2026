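; BPC_WeaponCollider is a component for BP_Weapon that turns melee hitbox overlaps into damage.
; On BeginPlay it binds to begin-overlap of the BoxComponent found on the weapon's WeaponModel.
; Overlaps ignore the weapon's attach parent and actors already in HittedActors on the owner's BPC_CombatComponent.
; New targets are added to that list, debug-printed and dealt random integer damage within the WeaponData min/max range.
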(event `self.ReceiveBeginPlay`
  (bind _asbp_weapon (cast `/Game/Blueprints/Weapons/BP_Weapon` (`KismetSystemLibrary.GetOuterObject` self)))
  (bind _output_get (set `self.Owner` _asbp_weapon))
  (bind _returnvalue (`Actor.GetComponentByClass` (`/Game/Blueprints/Weapons/BP_Weapon.weaponModel` _output_get) "/Script/Engine.BoxComponent"))
  (`/Engine/EditorBlueprintResources/StandardMacros.IsValid` _returnvalue
    (:`Is Valid`
      (add `PrimitiveComponent.OnComponentBeginOverlap` _returnvalue (delegate `BeginOverlap`)))))

(event `BeginOverlap`
  (params (OverlappedComponent :type "PrimitiveComponent Object Reference") (OtherActor :type "Actor Object Reference") (OtherComp :type "PrimitiveComponent Object Reference") (OtherBodyIndex :type Integer) (bFromSweep :type Boolean) (SweepResult :type "HitResult Structure (by ref)"))
  (bind (_weapondata_mindamage _weapondata_maxdamage) (break `/Game/Blueprints/Weapons/UtilWeaponData` (`/Game/Blueprints/Weapons/BP_Weapon.weaponData` (`self.Owner`))))
  (bind _returnvalue (`Actor.GetComponentByClass` (`Actor.GetOwner` (`self.Owner`)) "/Game/Blueprints/Weapons/Components/BPC_CombatComponent.BPC_CombatComponent_C"))
  (bind _hittedactors (`/Game/Blueprints/Weapons/Components/BPC_CombatComponent.HittedActors` _returnvalue))
  (if (!= OtherActor (`Actor.GetAttachParentActor` (`self.Owner`)))
    (if (`KismetSystemLibrary.IsValid` _returnvalue)
      (if (== (`KismetArrayLibrary.Array_Find` _hittedactors OtherActor) -1)
        (`KismetArrayLibrary.Array_Add` _hittedactors OtherActor)
        (`KismetSystemLibrary.PrintString` (`KismetSystemLibrary.GetDisplayName` OtherActor))
        (`GameplayStatics.ApplyDamage` OtherActor (`KismetMathLibrary.Conv_IntToDouble` (`KismetMathLibrary.RandomIntegerInRange` (`KismetMathLibrary.FTrunc` _weapondata_mindamage) (`KismetMathLibrary.FTrunc` _weapondata_maxdamage))))))))