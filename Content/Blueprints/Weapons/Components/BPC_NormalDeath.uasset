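; BPC_NormalDeath is an actor component that gives its owner a standard ragdoll death.
; Its Death event turns on physics simulation on the owner's mesh and disables capsule collision.
; After timed delays it sets the mesh to ignore all collision channels, then destroys the owner.
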(event `self.Death`
  (bind _owner (`self.owner`))
  (`PrimitiveComponent.SetSimulatePhysics` (`Character.Mesh` _owner) true)
  (`PrimitiveComponent.SetCollisionEnabled` (`Character.CapsuleComponent` _owner) "NoCollision")
  (`KismetSystemLibrary.Delay` 5.0)
  (`PrimitiveComponent.SetCollisionResponseToAllChannels` (`Character.Mesh` (`self.owner`)) "ECR_Ignore")
  (`KismetSystemLibrary.Delay` 2.0)
  (`Actor.K2_DestroyActor` (`self.owner`)))