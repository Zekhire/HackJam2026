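; Floor spike trap that activates when a Character enters its box and repeats its cycle while any Character remains inside.
; A timeline drives the spike Scene component's Z offset from its initial position, guarded by an IsActivated flag.
; DamagedCharacters acts as a pending-hit queue, refilled from the occupants each cycle and on entry.
; Timeline updates apply damage and remove entries, so occupants are hit per cycle rather than per frame.
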(event `self.ReceiveBeginPlay`
  (set `self.initSpikesTransform` (`SceneComponent.GetRelativeTransform` (`self.Scene`))))

(event `self.Box.OnComponentBeginOverlap`
  (params (OverlappedComponent :type "PrimitiveComponent Object Reference") (OtherActor :type "Actor Object Reference") (OtherComp :type "PrimitiveComponent Object Reference") (OtherBodyIndex :type Integer) (bFromSweep :type Boolean) (SweepResult :type "HitResult Structure (by ref)"))
  (bind _ascharacter (cast `Character` OtherActor))
  (`KismetArrayLibrary.Array_Add` (`self.characters`) _ascharacter)
  (`KismetArrayLibrary.Array_Add` (`self.damagedCharacters`) _ascharacter)
  (`self.TrapActivation`))

(event `self.Box.OnComponentEndOverlap`
  (params (OverlappedComponent :type "PrimitiveComponent Object Reference") (OtherActor :type "Actor Object Reference") (OtherComp :type "PrimitiveComponent Object Reference") (OtherBodyIndex :type Integer))
  (bind _ascharacter (cast `Character` OtherActor))
  (`KismetArrayLibrary.Array_RemoveItem` (`self.characters`) _ascharacter))

(event `TrapActivation`
  (bind _initspikestransform (`self.initSpikesTransform`))
  (if (not (`self.isActivated`))
    (set `self.isActivated` true)
    (if (> (`KismetArrayLibrary.Array_Length` (`self.characters`)) 0) :!label _label
      (for _array_element (`self.characters`)
        (if (== (`KismetArrayLibrary.Array_Find` (`self.damagedCharacters`) _array_element) -1)
          (`KismetArrayLibrary.Array_Add` (`self.damagedCharacters`) _array_element)))
      (bind (_direction _newtrack_0) (`Timeline|protrudingSpikesTimeline` :!via `PlayFromStart`)
        (:`Update`
          (`SceneComponent.K2_SetRelativeLocation` (`self.Scene`) (`KismetMathLibrary.MakeVector` (.x (.location _initspikestransform)) (.y (.location _initspikestransform)) (+ (* _newtrack_0 (`self.spikesHeightOffset`)) (.z (.location _initspikestransform)))) false false)
          (for _array_element_2 (`self.damagedCharacters`)
            (`GameplayStatics.ApplyDamage` _array_element_2 (`self.damage`))
            (`KismetArrayLibrary.Array_RemoveItem` (`self.damagedCharacters`) _array_element_2)))
        (:`Finished`
          (`KismetArrayLibrary.Array_Clear` (`self.damagedCharacters`))
          (goto _label)))
      (else
        (set `self.isActivated` false)))))

(fn `UserConstructionScript`)