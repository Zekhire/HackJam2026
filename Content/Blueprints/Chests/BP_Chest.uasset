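; BP_Chest is a one-time openable loot chest that presents a weapon to the player.
; Its Box overlap toggles input for BP_Player, so pressing E nearby opens it and disables further input.
; A timeline swings the lid by driving Scene1's roll.
; When it finishes, OBJ_WeaponFactory supplies data for ItemClass to spawn a BP_Weapon, which gains BPC_Acquirable, attaches to Scene2 and plays its acquirable animation.
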(event `self.Box.OnComponentBeginOverlap`
  (params (OverlappedComponent :type "PrimitiveComponent Object Reference") (OtherActor :type "Actor Object Reference") (OtherComp :type "PrimitiveComponent Object Reference") (OtherBodyIndex :type Integer) (bFromSweep :type Boolean) (SweepResult :type "HitResult Structure (by ref)"))
  (if (not (`self.isOpened`))
    (bind _asbp_player (cast `/Game/CustomCharacters/SkeletalMeshes/BP_Player` OtherActor))
    (`self.EnableInput` (`PlayerState.GetPlayerController` (`Pawn.PlayerState` _asbp_player)))))

(event `self.Box.OnComponentEndOverlap`
  (params (OverlappedComponent :type "PrimitiveComponent Object Reference") (OtherActor :type "Actor Object Reference") (OtherComp :type "PrimitiveComponent Object Reference") (OtherBodyIndex :type Integer))
  (if (not (`self.isOpened`))
    (bind _asbp_player (cast `/Game/CustomCharacters/SkeletalMeshes/BP_Player` OtherActor))
    (`self.DisableInput` (`PlayerState.GetPlayerController` (`Pawn.PlayerState` _asbp_player)))))

(event `Key|E`
  (params (Key :type "Key Structure"))
  (:`Pressed`
    (if (not (`self.isOpened`))
      (`self.DisableInput` null)
      (`self.OpenChest`))))

(event `OpenChest`
  (bind (_relativerotation_roll _relativerotation_pitch _relativerotation_yaw) (`KismetMathLibrary.BreakRotator` (`SceneComponent.RelativeRotation` (`self.Scene1`))))
  (set `self.isOpened` true)
  (bind (_direction _floattrack) (`Timeline|chestCoverRotationTimeline`)
    (:`Update`
      (`SceneComponent.K2_SetRelativeRotation` (`self.Scene1`) (`KismetMathLibrary.MakeRotator` (* _floattrack 90.0) _relativerotation_pitch _relativerotation_yaw) false false))
    (:`Finished`
      (bind _returnvalue (`|GenericCreateObject` "/Game/Blueprints/Weapons/OBJ_WeaponFactory.OBJ_WeaponFactory_C"))
      (bind (_value _returnvalue_2) (`BlueprintMapLibrary.Map_Find` (`/Game/Blueprints/Weapons/OBJ_WeaponFactory.Weapons` _returnvalue) (`|GetEnumeratorNameAsString` (`self.ItemClass`))))
      (if _returnvalue_2
        (bind _returnvalue_3 (`|SpawnActorFromClass` "/Game/Blueprints/Weapons/BP_Weapon.BP_Weapon_C" (`KismetMathLibrary.MakeTransform` (0.0 0.0 0.0)) "Undefined" "MultiplyWithRoot" self _value null))
        (bind _returnvalue_4 (`|AddComponentByClass` _returnvalue_3 "/Game/Blueprints/Weapons/Components/BPC_Acquirable.BPC_Acquirable_C"))
        (`self.K2_AttachToComponent` _returnvalue_3 (`self.Scene2`) "None" "KeepRelative" "KeepRelative" "KeepRelative" true)
        (`/Game/Blueprints/Weapons/Components/BPC_Acquirable.AcquirableAnimation` _returnvalue_4)))))

(fn `UserConstructionScript`)