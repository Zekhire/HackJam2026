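; Character component for a black scribble effect that hides the owner's mesh while keeping its bones animating.
; BeginPlay generates randomly offset points around random bones, then Scribble repeats each second, destroying the owner's static mesh components, re-jittering points and picking pairs in DrawLines.
; The stretched-cube line spawning is disconnected, so nothing is drawn.
; An alternative Scrawl loop attaching jittering cubes to random sockets also has disconnected setup.
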(event `self.ReceiveBeginPlay`
  (bind _ascharacter (cast `Character` (`KismetSystemLibrary.GetOuterObject` self)))
  (bind _output_get (set `self.characterOwner` _ascharacter))
  (bind _mesh (`Character.Mesh` _output_get))
  (set `SkinnedMeshComponent.VisibilityBasedAnimTickOption` "AlwaysTickPoseAndRefreshBones" _mesh)
  (`SceneComponent.SetVisibility` _mesh false false)
  (bind _output_get_2 (set `self.allBones` (`SceneComponent.GetAllSocketNames` (`Character.Mesh` (`self.characterOwner`)))))
  (`KismetArrayLibrary.Array_Shuffle` _output_get_2)
  (`self.GeneratePoints`)
  (`self.Scribble`))

(event `Scribble`
  (for _array_element (`Actor.K2_GetComponentsByClass` (`self.characterOwner`) "/Script/Engine.StaticMeshComponent")
    (`self.K2_DestroyComponent` _array_element))
  (`self.UpdatePoints`)
  (`self.DrawLines`)
  (`KismetSystemLibrary.K2_SetTimerDelegate` (delegate `KeepScribbling`) 1.0 true))

(event `KeepScribbling`
  (`self.Scribble`))

(event `Scrawl`
  (bind _mesh (`Character.Mesh` (`self.characterOwner`)))
  (for _array_element (`self.blackBlocks`)
    (`SceneComponent.K2_SetRelativeTransform` _array_element (`KismetMathLibrary.MakeTransform` (`KismetMathLibrary.MakeVector` (`KismetMathLibrary.RandomFloatInRange` 1.0 10.0) (`KismetMathLibrary.RandomFloatInRange` 1.0 10.0) (`KismetMathLibrary.RandomFloatInRange` 1.0 10.0)) (`KismetMathLibrary.MakeRotator` (`KismetMathLibrary.RandomFloatInRange` -180.0 180.0) (`KismetMathLibrary.RandomFloatInRange` -180.0 180.0) (`KismetMathLibrary.RandomFloatInRange` -180.0 180.0)) (`KismetMathLibrary.MakeVector` (`KismetMathLibrary.RandomFloatInRange` 0.05 0.2) (`KismetMathLibrary.RandomFloatInRange` 0.05 0.2) (`KismetMathLibrary.RandomFloatInRange` 0.05 0.2))) false false)
    (`SceneComponent.K2_AttachToComponent` _array_element _mesh (`KismetArrayLibrary.Array_Random` (`SceneComponent.GetAllSocketNames` _mesh)) "KeepRelative" "KeepRelative" "KeepRelative" true)
    (`KismetSystemLibrary.K2_SetTimerDelegate` (delegate `ScrawlFinished`) 0.2)))

(event `ScrawlFinished`
  (`self.Scrawl`))

(fn `DrawLines`
  (locals (indexA :type Integer) (indexB :type Integer))
  (bind _points (`self.points`))
  (for _ (range 1 (+ (`self.nLines`) 1))
    (set `local.indexA` (`.OutIndex` (`KismetArrayLibrary.Array_Random` _points)))
    (set `local.indexB` (`.OutIndex` (`KismetArrayLibrary.Array_Random` _points)))
    (while (== (`local.indexA`) (`local.indexB`))
      (set `local.indexB` (`.OutIndex` (`KismetArrayLibrary.Array_Random` (`self.points`)))))))

(fn `GeneratePoints`
  (locals (randomBone :type Name))
  (bind _returnvalue (`KismetMathLibrary.RandomFloatInRange` 0.05 0.2))
  (bind _returnvalue_2 (`KismetMathLibrary.RandomFloatInRange` -10.0 10.0))
  (bind _returnvalue_3 (`KismetMathLibrary.RandomFloatInRange` -180.0 180.0))
  (bind (_returnvalue_location _returnvalue_rotation _returnvalue_scale) (`KismetMathLibrary.BreakTransform` (`KismetMathLibrary.MakeTransform` (`KismetMathLibrary.MakeVector` _returnvalue_2 _returnvalue_2 _returnvalue_2) (`KismetMathLibrary.MakeRotator` _returnvalue_3 _returnvalue_3 _returnvalue_3) (`KismetMathLibrary.MakeVector` _returnvalue _returnvalue _returnvalue))))
  (for _ (range 1 (+ (`self.nPoints`) 1))
    (bind _output_get (set `local.randomBone` (`KismetArrayLibrary.Array_Random` (`self.allBones`))))
    (bind (_returnvalue_location_2 _returnvalue_rotation_2 _returnvalue_scale_2) (`KismetMathLibrary.BreakTransform` (`SkinnedMeshComponent.GetBoneTransform` (`Character.Mesh` (`self.characterOwner`)) _output_get "RTS_World")))
    (`KismetArrayLibrary.Array_Add` (`self.points`) (make `/Game/Blueprints/Components/Struct_ScribblePoint` "None" (`KismetMathLibrary.MakeTransform` _returnvalue_location _returnvalue_rotation _returnvalue_scale) (`KismetMathLibrary.MakeTransform` (+ _returnvalue_location _returnvalue_location_2) (`KismetMathLibrary.ComposeRotators` _returnvalue_rotation _returnvalue_rotation_2) (+ _returnvalue_scale _returnvalue_scale_2))))))

(fn `UpdatePoints`
  (bind _returnvalue (`KismetMathLibrary.RandomFloatInRange` 0.05 0.2))
  (bind _returnvalue_2 (`KismetMathLibrary.RandomFloatInRange` -10.0 10.0))
  (bind _returnvalue_3 (`KismetMathLibrary.RandomFloatInRange` -180.0 180.0))
  (bind (_returnvalue_location _returnvalue_rotation _returnvalue_scale) (`KismetMathLibrary.BreakTransform` (`KismetMathLibrary.MakeTransform` (`KismetMathLibrary.MakeVector` _returnvalue_2 _returnvalue_2 _returnvalue_2) (`KismetMathLibrary.MakeRotator` _returnvalue_3 _returnvalue_3 _returnvalue_3) (`KismetMathLibrary.MakeVector` _returnvalue _returnvalue _returnvalue))))
  (for (_array_element _array_index) (`self.points`)
    (bind (_returnvalue_location_2 _returnvalue_rotation_2 _returnvalue_scale_2) (`KismetMathLibrary.BreakTransform` (`SkinnedMeshComponent.GetBoneTransform` (`Character.Mesh` (`self.characterOwner`)) (break `/Game/Blueprints/Components/Struct_ScribblePoint` _array_element) "RTS_World")))
    (`KismetArrayLibrary.Array_Set` (`self.points`) _array_index (make `/Game/Blueprints/Components/Struct_ScribblePoint` (break `/Game/Blueprints/Components/Struct_ScribblePoint` _array_element) (`KismetMathLibrary.MakeTransform` _returnvalue_location _returnvalue_rotation _returnvalue_scale) (`KismetMathLibrary.MakeTransform` (+ _returnvalue_location _returnvalue_location_2) (`KismetMathLibrary.ComposeRotators` _returnvalue_rotation _returnvalue_rotation_2) (+ _returnvalue_scale _returnvalue_scale_2))))))