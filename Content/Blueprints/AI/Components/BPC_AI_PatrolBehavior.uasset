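; AI behavior component that makes its owning character patrol around its start location and chase nearby players.
; Patrol moves to random reachable points within a radius, pausing on a timer after each successful arrival.
; Every tick it finds the closest BP_Player; within detection range it reissues AIMoveTo toward them and calls BPC_CombatComponent's Attack on arrival.
; When no player is in range, it drops the chase and resumes patrolling.
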(event `self.ReceiveBeginPlay`
  (bind _ascharacter (cast `Character` (`KismetSystemLibrary.GetOuterObject` self)))
  (bind _output_get (set `self.ownerCharacter` _ascharacter))
  (set `self.initLocation` (`Actor.K2_GetActorLocation` _output_get))
  (bind _asaicontroller (cast `AIController` (`Pawn.GetController` _output_get)))
  (set `self.AIController` _asaicontroller)
  (`self.StartPatrol`))

(event `self.ReceiveTick`
  (params (DeltaSeconds :type "Float (single-precision)"))
  (`self.Update` DeltaSeconds))

(event `StartPatrol`
  (`KismetSystemLibrary.K2_ClearAndInvalidateTimerHandle` (`self.PatrolTimer`))
  (bind _output_get (set `self.patrolLocation` (`NavigationSystemV1.K2_GetRandomReachablePointInRadius` (`self.initLocation`) (`self.patrolRadius`) null null)))
  (`|AIMoveTo` (`self.ownerCharacter`) _output_get null 50.0
    (:`OnSuccess`
      (bind _returnvalue (`KismetSystemLibrary.K2_SetTimerDelegate` (delegate `PatrolAfterDestination`) 3.0))
      (set `self.PatrolTimer` _returnvalue))))

(event `PatrolAfterDestination`
  (`self.StartPatrol`))

(event `Update`
  (params (deltaSeconds :type "Float (double-precision)"))
  (bind _theclosestplayer (`self.GetTheClosestPlayer`))
  (if (`KismetSystemLibrary.IsValid` _theclosestplayer)
    (if (<= (`KismetMathLibrary.Vector_Distance` (`Actor.K2_GetActorLocation` _theclosestplayer) (`Actor.K2_GetActorLocation` (`self.ownerCharacter`))) (`self.detectionRadius`))
      (if (not (== (`self.playerTarget`) _theclosestplayer))
        (`self.StartChase` _theclosestplayer)
        (else
          (`self.ContinueChase`)))
      (else
        (if (`self.isChasing`) :!label _label
          (`self.ReturnToPatrol`))))
    (else
      (goto _label))))

(event `StartChase`
  (params (playerTarget :type "/Game/CustomCharacters/SkeletalMeshes/BP_Player Object Reference"))
  (set `self.playerTarget` playerTarget)
  (if (not (`self.isChasing`))
    (set `self.isChasing` true)
    (`Controller.StopMovement` (`self.AIController`))
    (`KismetSystemLibrary.K2_ClearAndInvalidateTimerHandle` (`self.PatrolTimer`)))
  (`self.ContinueChase`))

(event `ContinueChase`
  (bind _returnvalue (`Actor.GetComponentByClass` (`self.ownerCharacter`) "/Game/Blueprints/Weapons/Components/BPC_CombatComponent.BPC_CombatComponent_C"))
  (`|AIMoveTo` (`self.ownerCharacter`) (0.0 0.0 0.0) (`self.playerTarget`) 50.0 true
    (:`OnSuccess`
      (if (`KismetSystemLibrary.IsValid` _returnvalue)
        (`/Game/Blueprints/Weapons/Components/BPC_CombatComponent.Attack` _returnvalue)))))

(event `ReturnToPatrol`
  (set `self.isChasing` false)
  (set `self.playerTarget` null)
  (`Controller.StopMovement` (`self.AIController`))
  (`self.StartPatrol`))

(fn `GetTheClosestPlayer`
  (returns (theClosestPlayer :type "/Game/CustomCharacters/SkeletalMeshes/BP_Player Object Reference"))
  (locals (potentialTheClosestPlayer :type "/Game/CustomCharacters/SkeletalMeshes/BP_Player Object Reference"))
  (bind _outactors (`GameplayStatics.GetAllActorsOfClass` "/Game/CustomCharacters/SkeletalMeshes/BP_Player.BP_Player_C"))
  (if (> (`KismetArrayLibrary.Array_Length` _outactors) 0)
    (set `local.potentialTheClosestPlayer` (`|GetArrayItem` _outactors))
    (bind _returnvalue (`KismetArrayLibrary.Array_Length` _outactors))
    (if (> _returnvalue 1)
      (for _index (range 1 _returnvalue)
        (bind _output (`|GetArrayItem` _outactors _index))
        (if (< (`KismetMathLibrary.Vector_Distance` (`Actor.K2_GetActorLocation` _output) (`Actor.K2_GetActorLocation` (`self.ownerCharacter`))) (`KismetMathLibrary.Vector_Distance` (`Actor.K2_GetActorLocation` (`local.potentialTheClosestPlayer`)) (`Actor.K2_GetActorLocation` (`self.ownerCharacter`))))
          (set `local.potentialTheClosestPlayer` _output)))))
  (return (`local.potentialTheClosestPlayer`)))