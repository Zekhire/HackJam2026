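; Enemy AI character Blueprint that provides a looping random patrol around its spawn location.
; BeginPlay caches the starting position, and the Patrol event moves the pawn to random reachable points within a maximum radius of it.
; A successful move waits briefly before Patrol calls itself again, while a failed move retries without the delay.
; Nothing connected in this Blueprint starts the loop.
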(event `self.ReceiveBeginPlay`
  (set `self.initPosition` (`self.K2_GetActorLocation` self)))

(event `Patrol`
  (`|AIMoveTo` self (`NavigationSystemV1.K2_GetRandomReachablePointInRadius` (`self.initPosition`) (`self.maxRadiusPatrol`) null null) null 70.0
    (:`OnSuccess`
      (`KismetSystemLibrary.Delay` 3.0))
    (:`OnFail`
      _))
  (`self.Patrol`))

(fn `UserConstructionScript`)