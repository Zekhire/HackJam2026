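; Actor component that lets the third-person character swap between masks worn on its mesh.
; On BeginPlay it casts its owner to BP_ThirdPersonCharacter, adds a static mesh component, sets the first mask and attaches it to a named socket on the character's mesh.
; Gamepad D-pad presses call WearMask, which replaces that component's static mesh with the matching entry from the mask array.
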(event `self.ReceiveBeginPlay`
  ; Get Owner Actor Reference
  (bind _asbp_third_person_character (cast `/Game/ThirdPerson/Blueprints/BP_ThirdPersonCharacter` (`self.GetOwner`)))
  (bind _output_get (set `self.Owner_Actor` _asbp_third_person_character))
  (set `self.MeshComponent` (`Actor.GetComponentByClass` _output_get "/Script/Engine.MeshComponent"))
  ; Initialize Mask Component
  (bind _returnvalue (`|AddComponentByClass` :`self` _output_get :`Class` "/Script/Engine.StaticMeshComponent"))
  (set `self.ActiveMaskComponent` _returnvalue)
  (`self.WearMask` 0)
  ; Wear Mask On Owner
  (`SceneComponent.K2_AttachToComponent` (`self.ActiveMaskComponent`) (`self.MeshComponent`) (`self.Socket Name`) "KeepRelative" "KeepRelative" "KeepRelative" true))

(event `WearMask`
  (params (MaskId :type Integer))
  (`StaticMeshComponent.SetStaticMesh` (`self.ActiveMaskComponent`) (`|GetArrayItem` (`self.MaskArr`) MaskId)))

(event `Key|Gamepad_DPad_Up`
  (params (Key :type "Key Structure"))
  (:`Pressed`
    (`self.WearMask` 0)))

(event `Key|Gamepad_DPad_Down`
  (params (Key :type "Key Structure"))
  (:`Pressed`
    (`self.WearMask` 1)))

(event `Key|Gamepad_DPad_Right`
  (params (Key :type "Key Structure"))
  (:`Pressed`
    (`self.WearMask` 2)))

(event `Key|Gamepad_DPad_Left`
  (params (Key :type "Key Structure"))
  (:`Pressed`
    (`self.WearMask` 3)))