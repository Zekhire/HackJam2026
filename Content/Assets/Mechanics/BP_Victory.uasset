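; BP_Victory is the win-condition actor that ends the game based on progress along the BP_Spline path.
; Each Tick it calls GetProgress, which divides that spline actor's DistanceAlongSpline by the spline length, and compares the raw ratio, unscaled, against 100.
; When the threshold is met it adds the UW_EndGame widget, with no once-only guard, and loads LVL_MainMenu after a delay.
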(event `self.ReceiveTick`
  (params (DeltaSeconds :type "Float (single-precision)"))
  (bind _progress (`self.GetProgress`))
  (if (>= _progress 100.0)
    (`|ExecutionSequence`
      (:`then_0`
        (bind _returnvalue (`|CreateWidget` "/Game/Assets/UI/UW_EndGame.UW_EndGame_C" (`GameplayStatics.GetPlayerController` 0)))
        (`UserWidget.AddToViewport` _returnvalue 0))
      (:`then_1`
        (`KismetSystemLibrary.Delay` 5.0)
        (`GameplayStatics.OpenLevel` "LVL_MainMenu")))))

(fn `GetProgress`
  (returns (Progress :type "Float (double-precision)"))
  (bind _returnvalue (`GameplayStatics.GetActorOfClass` "/Game/Blueprints/Spline/BP_Spline.BP_Spline_C"))
  (return (/ (`/Game/Blueprints/Spline/BP_Spline.distanceAlongSpline` _returnvalue) (`SplineComponent.GetSplineLength` (`/Game/Blueprints/Spline/BP_Spline.Spline` _returnvalue)))))

(fn `UserConstructionScript`)