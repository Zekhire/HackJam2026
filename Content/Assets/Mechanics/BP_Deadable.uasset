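; BP_Deadable provides a KillPlayer event that runs the player's death and game-over sequence.
; KillPlayer stops the BP_Spline tick, ragdolls the player's mesh with WorldStatic blocking, and destroys all enemy ring generators.
; It then shows the UW_EndGame widget and opens the main menu level after a short delay.
; Nothing connected in this Blueprint triggers KillPlayer.
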(event `self.ReceiveBeginPlay`)

(event `KillPlayer`
  (`|ExecutionSequence`
    (:`then_0`
      (bind _returnvalue (`GameplayStatics.GetActorOfClass` "/Game/Blueprints/Spline/BP_Spline.BP_Spline_C"))
      (`self.SetActorTickEnabled` _returnvalue false)
      (bind _asbp_player (cast `/Game/CustomCharacters/SkeletalMeshes/BP_Player` (`GameplayStatics.GetPlayerPawn` 0)))
      (bind _mesh (`Character.Mesh` _asbp_player))
      (`PrimitiveComponent.SetSimulatePhysics` _mesh true)
      (`PrimitiveComponent.SetCollisionResponseToChannel` _mesh "ECC_WorldStatic" "ECR_Block"))
    (:`then_1`
      (bind _outactors (`GameplayStatics.GetAllActorsOfClass` "/Game/Assets/Mechanics/BP_EnemyRingsGenerator.BP_EnemyRingsGenerator_C"))
      (for _array_element _outactors
        (`self.K2_DestroyActor` _array_element)))
    (:`then_2`
      (bind _returnvalue_2 (`|CreateWidget` "/Game/Assets/UI/UW_EndGame.UW_EndGame_C" (`GameplayStatics.GetPlayerController` 0)))
      (`UserWidget.AddToViewport` _returnvalue_2 0))
    (:`then_3`
      (`KismetSystemLibrary.Delay` 5.0)
      (`GameplayStatics.OpenLevel` "LVL_MainMenu"))))

(fn `UserConstructionScript`)