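; Player component that fires rings of two colors from the gamepad triggers, through a BP_RingsGenerator it spawns at BeginPlay.
; The right and left triggers call GenerateRing with opposite color flags, both marked as non-enemy.
; Each shot starts a shared cooldown, which Tick clears once accumulated time reaches Period.
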(event `self.ReceiveBeginPlay`
  (bind _returnvalue (`|SpawnActorFromClass` "/Game/Assets/Mechanics/BP_RingsGenerator.BP_RingsGenerator_C" (`KismetMathLibrary.MakeTransform` (0.0 0.0 0.0)) "Undefined" "MultiplyWithRoot" null null))
  (set `self.Rings Generator` _returnvalue))

(event `self.ReceiveTick`
  (params (DeltaSeconds :type "Float (single-precision)"))
  (if (`self.Cooldown`)
    (bind _output_get (set `self.TimeAcc` (+ (`self.TimeAcc`) DeltaSeconds)))
    (if (>= _output_get (`self.Period`))
      (set `self.Cooldown` false)
      (set `self.TimeAcc` 0.0))))

(event `Key|Gamepad_RightTrigger`
  (params (Key :type "Key Structure"))
  (:`Pressed`
    (if (not (`self.Cooldown`))
      (`/Game/Assets/Mechanics/BP_RingsGenerator.GenerateRing` (`self.Rings Generator`) false false)
      (set `self.Cooldown` true))))

(event `Key|Gamepad_LeftTrigger`
  (params (Key :type "Key Structure"))
  (:`Pressed`
    (if (not (`self.Cooldown`))
      (`/Game/Assets/Mechanics/BP_RingsGenerator.GenerateRing` (`self.Rings Generator`) true false)
      (set `self.Cooldown` true))))