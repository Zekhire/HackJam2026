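; Enemy ring spawner that plays a timed, data-driven sequence of enemy rings.
; On BeginPlay it spawns a BP_RingsGenerator, then Tick accumulates elapsed time and loads the next DT_Sequence row by index through the table's row names.
; When that row's timestamp is reached, a Ring action tells the generator to emit an enemy ring colored by the row's Variant, then advances to the following row.
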(event `self.ReceiveBeginPlay`
  (bind _returnvalue (`|SpawnActorFromClass` "/Game/Assets/Mechanics/BP_RingsGenerator.BP_RingsGenerator_C" (`KismetMathLibrary.MakeTransform` (0.0 0.0 0.0)) "Undefined" "MultiplyWithRoot" null null))
  (set `self.RingsGenerator` _returnvalue))

(event `self.ReceiveTick`
  (params (DeltaSeconds :type "Float (single-precision)"))
  (bind (_nextexpectedaction_timestamp _nextexpectedaction_action _nextexpectedaction_variant) (break `/Game/Assets/TextAssets/ST_Sequence` (`self.NextExpectedAction`)))
  (`|ExecutionSequence`
    (:`then_0`
      (set `self.TimeProgress` (+ (`self.TimeProgress`) DeltaSeconds)))
    (:`then_7`
      (if (`self.bNext`)
        (bind _out_row (`self.GetSequenceRow` (`self.SequenceRowId`)))
        (set `self.NextExpectedAction` _out_row)
        (set `self.bNext` false)
        (elif (>= (`self.TimeProgress`) _nextexpectedaction_timestamp)
          (switch `string` _nextexpectedaction_action
            (:`ring`
              (`/Game/Assets/Mechanics/BP_RingsGenerator.GenerateRing` (`self.RingsGenerator`) (`KismetMathLibrary.Conv_IntToBool` _nextexpectedaction_variant) true)
              (set `self.bNext` true)
              (`/Engine/EditorBlueprintResources/StandardMacros.IncrementInt` (`self.SequenceRowId`)))))))))

(fn `GetSequenceRow`
  (params (SequenceRowId :type Integer))
  (returns (`Out Row` :type "/Game/Assets/TextAssets/ST_Sequence Structure"))
  (bind _outrownames (`DataTableFunctionLibrary.GetDataTableRowNames` "/Game/Assets/TextAssets/DT_Sequence.DT_Sequence"))
  (bind _returnvalue (`|GetDataTableRow` "/Game/Assets/TextAssets/DT_Sequence.DT_Sequence" (`|GetArrayItem` _outrownames SequenceRowId))
    (:`then`
      (return _returnvalue))))

(fn `UserConstructionScript`)