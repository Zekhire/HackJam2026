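; Mask component that lets its owning Character wear and unwear a mask object.
; Initialization caches the outer object as the owner and sets an initialized flag, only if it is a Character.
; WearMask stores the given mask and calls its OnWear with the owner, delegating the effect to the mask.
; UnwearMask calls OnUnwear on the stored mask without clearing the reference.
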(event `self.ReceiveTick`
  (params (DeltaSeconds :type "Float (single-precision)")))

(event `Initialization`
  (bind _ascharacter (cast `Character` (`KismetSystemLibrary.GetOuterObject` self)))
  (set `self.OwnerCharacter` _ascharacter)
  (set `self.Initialized` true))

(event `WearMask`
  (params (MaskObjectToWear :type "/Game/Assets/Mechanics/BP_Mask Object Reference"))
  (bind _output_get (set `self.Mask` MaskObjectToWear))
  (`/Game/Assets/Mechanics/BP_Mask.OnWear` _output_get (`self.OwnerCharacter`)))

(event `UnwearMask`
  (`/Game/Assets/Mechanics/BP_Mask.OnUnwear` (`self.Mask`)))