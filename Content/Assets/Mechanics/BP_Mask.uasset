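; BP_Mask is a wearable mask actor that can be attached to and detached from another actor's mesh.
; Initialization applies the configured static mesh, and OnWear attaches the mask to the parent's mesh at a named socket, keeping relative transforms.
; OnUnwear detaches it.
; Both then call WearMask or UnwearMask, separate events that currently only print debug strings as placeholders for mask effects.
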(event `self.ReceiveTick`
  (params (DeltaSeconds :type "Float (single-precision)")))

(event `Initialization`
  (`StaticMeshComponent.SetStaticMesh` (`self.MaskStaticMeshComponent`) (`self.MaskStaticMesh`)))

(event `OnWear`
  (params (ParentActor :type "Character Object Reference"))
  (`self.K2_AttachToComponent` self (`Character.Mesh` ParentActor) (`self.Socket Name`) "KeepRelative" "KeepRelative" "KeepRelative" true)
  (`self.SetOwner` self null)
  (`self.WearMask`))

(event `OnUnwear`
  (`self.K2_DetachFromActor` "KeepRelative")
  (`self.UnwearMask`))

(event `WearMask`
  (`KismetSystemLibrary.PrintString` "WEAR"))

(event `UnwearMask`
  (`KismetSystemLibrary.PrintString` "UNWEAR"))

(fn `UserConstructionScript`)