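; BP_Ring is a white or black ring actor, set up as either an enemy or a player ring.
; Once initialized, Tick shrinks enemy rings or grows player rings, destroying them at scale limits.
; When an enemy ring overlaps a collidable player ring, matching colors destroy both, while a mismatch destroys all player rings, each with a sound.
; An enemy ring overlapping BP_Player calls KillPlayer on the first BP_Deadable found during initialization.
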(event `self.ReceiveBeginPlay`)

(event `self.ReceiveTick`
  (params (DeltaSeconds :type "Float (single-precision)"))
  (if (`self.bInitialized`)
    (if (`self.bEnemy`)
      (`self.DecreaseScale` DeltaSeconds)
      (else
        (`self.IncreaseScale` DeltaSeconds)))))

(event `Initialization`
  (params (Color :type Boolean) (`Enemy?` :type Boolean))
  (set `self.bEnemy` `Enemy?`)
  (bind _output_get (set `self.Color` Color))
  (if _output_get
    (`PrimitiveComponent.SetMaterial` (`self.RingStaticMeshComponent`) 0 "/Game/Assets/Rings/M_White.M_White")
    (else
      (`PrimitiveComponent.SetMaterial` (`self.RingStaticMeshComponent`) 0 "/Game/Assets/Rings/M_Black.M_Black")))
  (if (`self.bEnemy`)
    (set `self.Scale` 3.0)
    (else
      (set `self.Scale` (`self.MinScaleToRemove`))))
  (`self.GetBPDeadable`)
  (set `self.bInitialized` true))

(event `DecreaseScale`
  (params (DeltaSeconds :type "Float (double-precision)"))
  (if (>= (`self.Scale`) (`self.MinScaleToRemove`))
    (bind _output_get (set `self.Scale` (- (`self.Scale`) (* DeltaSeconds 0.5))))
    (`SceneComponent.SetWorldScale3D` (`self.RingStaticMeshComponent`) (`KismetMathLibrary.MakeVector` _output_get _output_get 1.0))
    (else
      (`self.K2_DestroyActor`))))

(event `IncreaseScale`
  (params (DeltaSeconds :type "Float (double-precision)"))
  (if (<= (`self.Scale`) 10.0)
    (bind _output_get (set `self.Scale` (+ (`self.Scale`) (* DeltaSeconds 0.5))))
    (`SceneComponent.SetWorldScale3D` (`self.RingStaticMeshComponent`) (`KismetMathLibrary.MakeVector` _output_get _output_get 1.0))
    (else
      (`self.K2_DestroyActor`))))

(event `self.Sphere.OnComponentBeginOverlap`
  (params (OverlappedComponent :type "PrimitiveComponent Object Reference") (OtherActor :type "Actor Object Reference") (OtherComp :type "PrimitiveComponent Object Reference") (OtherBodyIndex :type Integer) (bFromSweep :type Boolean) (SweepResult :type "HitResult Structure (by ref)"))
  (if (`self.bInitialized`)
    (bind _asbp_ring (cast `/Game/Assets/Rings/BP_Ring` OtherActor)
      (:`then`
        (bind _output_get (set `self.RingCollision` _asbp_ring))
        (if (`/Game/Assets/Rings/BP_Ring.bInitialized` _output_get)
          (if (`/Game/Assets/Rings/BP_Ring.Collidable` _output_get)
            ; Dla uproszczenia tylko wrogie pierścienie powodują niszczenie się siebie nawzajem
            (if (`self.bEnemy`)
              (if (not (`/Game/Assets/Rings/BP_Ring.bEnemy` (`self.RingCollision`)))
                (set `/Game/Assets/Rings/BP_Ring.Collidable` false (`self.RingCollision`))
                (if (== (`/Game/Assets/Rings/BP_Ring.Color` (`self.RingCollision`)) (`self.Color`))
                  (bind _returnvalue (`self.NewFunction`))
                  (`GameplayStatics.PlaySound2D` "/Game/Assets/Audio/Signal_Positive_Ceramic_C.Signal_Positive_Ceramic_C" 1.0 1.0 0.0 null null)
                  (`self.K2_DestroyActor`)
                  (`self.K2_DestroyActor` (`self.RingCollision`))
                  (else
                    (bind _returnvalue_2 (`self.NewFunction`))
                    (`GameplayStatics.PlaySound2D` "/Game/Assets/Audio/Signal_Negative_Metal_Fence_A.Signal_Negative_Metal_Fence_A" 1.0 1.0 0.0 null null)
                    ; Pomylenie koloru przez Gracza powoduje usunięcie wszystkich jego pierścieni
                    (bind _outactors (`GameplayStatics.GetAllActorsOfClass` "BP_Ring_C"))
                    (for _array_element _outactors
                      (if (not (`/Game/Assets/Rings/BP_Ring.bEnemy` _array_element))
                        (`self.K2_DestroyActor` _array_element))))))))))
      (:`CastFailed`
        (if (`self.bEnemy`)
          (cast `/Game/CustomCharacters/SkeletalMeshes/BP_Player` OtherActor)
          (`KismetSystemLibrary.PrintString` "AAAA")
          (`/Game/Assets/Mechanics/BP_Deadable.KillPlayer` (`self.deadableActor`)))))))

(fn `GetBPDeadable`
  (returns (DeadableActorLocal :type "/Game/Assets/Mechanics/BP_Deadable Object Reference"))
  (bind _outactors (`GameplayStatics.GetAllActorsOfClass` "/Game/Assets/Mechanics/BP_Deadable.BP_Deadable_C"))
  (for _array_element _outactors
    (set `self.deadableActor` _array_element)
    (break))
  (return (`self.deadableActor`)))

(fn `NewFunction`
  (returns (ReturnValue :type String))
  (bind _ringcollision (`self.RingCollision`))
  (if (`self.bEnemy`)
    (set `self.eString` "Enemy")
    (else
      (set `self.eString` "Player")))
  (if (`self.Color`)
    (set `self.cString` "White")
    (else
      (set `self.cString` "Black")))
  (if (`/Game/Assets/Rings/BP_Ring.bEnemy` _ringcollision)
    (set `self.eString_0` "Enemy")
    (else
      (set `self.eString_0` "Player")))
  (if (`/Game/Assets/Rings/BP_Ring.Color` _ringcollision)
    (set `self.cString_0` "White")
    (else
      (set `self.cString_0` "Black")))
  (return (`KismetStringLibrary.Concat_StrStr` (`KismetSystemLibrary.GetDisplayName` self) "bedacy:" (`self.eString`) " i mający kolor:" (`self.cString`) " Spowodował kolizję z   " (`KismetSystemLibrary.GetDisplayName` _ringcollision) "bedacy:   " (`self.eString_0`) " i mający kolor:  " (`self.cString_0`))))

(fn `UserConstructionScript`)